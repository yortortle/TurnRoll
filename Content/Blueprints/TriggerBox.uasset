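; Trigger box actor that signals when any actor enters or leaves it and toggles a text render's visibility.
; Begin and end overlap set the IntTrigger flag, then share one branch on it.
; Both branches toggle the text, with entry calling the Eventdisp dispatcher and exit calling Eventdisptwo.
; The overlapping actor is not filtered.
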(event `self.ReceiveActorBeginOverlap`
  (params (OtherActor :type "Actor Object Reference"))
  (set `self.IntTrigger` true)
  (if (`self.IntTrigger`) :!label _label
    (`SceneComponent.ToggleVisibility` (`self.TextRender`) false)
    (`self.eventdisp`)
    (else
      (`SceneComponent.ToggleVisibility` (`self.TextRender`) false)
      (`self.eventdisptwo`))))

(event `self.ReceiveActorEndOverlap`
  (params (OtherActor :type "Actor Object Reference"))
  (set `self.IntTrigger` false)
  (goto _label))

(fn `UserConstructionScript`)
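; YortBP is a character Blueprint whose only logic here opens the pause menu when Tab is released.
; It pauses the game, adds a Pause_Main widget to the viewport, switches to UI-only input and shows the mouse cursor.
; It then passes the first two PartyMembers from MyGameInstance to the widget as CharacterTarget and PartyMember2, printing an error if the cast fails.
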(event `Key|Tab`
  (params (Key :type "Key Structure"))
  (bind _returnvalue (`GameplayStatics.GetPlayerController` 0))
  (:`Released`
    (`GameplayStatics.SetGamePaused` true)
    (bind _returnvalue_2 (`|CreateWidget` "/Game/Blueprints/UI/Pause_Main.Pause_Main_C"))
    (`UserWidget.AddToViewport` _returnvalue_2 0)
    (`WidgetBlueprintLibrary.SetInputMode_UIOnlyEx` _returnvalue null)
    (set `PlayerController.bShowMouseCursor` true _returnvalue)
    (bind _asmy_game_instance (cast `MyGameInstance` (`GameplayStatics.GetGameInstance`))
      (:`then`
        (bind _partymembers (`MyGameInstance.PartyMembers` _asmy_game_instance))
        (set `/Game/Blueprints/UI/Pause_Main.Character Target` (`|GetArrayItem` _partymembers) _returnvalue_2)
        (set `/Game/Blueprints/UI/Pause_Main.PartyMember2` (`|GetArrayItem` _partymembers 1) _returnvalue_2))
      (:`CastFailed`
        (`KismetSystemLibrary.PrintString` "maincharacter cast to game instance failed")))))

(fn `UserConstructionScript`)